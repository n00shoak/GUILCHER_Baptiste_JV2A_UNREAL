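; BP_Lazer is a terrain laser hazard that toggles on and off and sends the game to MAP_SideScroller on contact.
; BeginPlay runs an endless Delay loop that alternates the Beam's visibility and the IsActive flag at five-second intervals.
; While IsActive is true, any overlap with the Box opens that level by name, with no check on the overlapping actor.
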(event OnComponentBeginOverlap(Box)
  (params (OverlappedComponent :type Primitive%20Component%20Object%20Reference) (OtherActor :type Actor%20Object%20Reference) (OtherComp :type Primitive%20Component%20Object%20Reference) (OtherBodyIndex :type Integer) (bFromSweep :type Boolean) (SweepResult :type Hit%20Result%20Structure%20%28by%20ref%29))
  (if (Variables|Default|GetIsActive)
    (Game|OpenLevel(byName) "MAP_SideScroller")))

(event EventBeginPlay
  (Utilities|FlowControl|Delay 5.0 :!label _label)
  (Rendering|SetVisibility (Variables|Default|GetBeam) false false)
  (Variables|Default|SetIsActive false)
  (Utilities|FlowControl|Delay 5.0)
  (Rendering|SetVisibility (Variables|Default|GetBeam) true false)
  (Variables|Default|SetIsActive true)
  (goto _label))

(fn ConstructionScript)